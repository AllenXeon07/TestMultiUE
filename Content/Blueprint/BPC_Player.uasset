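; Player controller that handles multiplayer session hosting, browsing and joining through Advanced Sessions nodes.
; On BeginPlay it creates the WB_HUD widget, shows the mouse cursor and passes itself to the HUD.
; Creating a session opens ThirdPersonMap as a listen server.
; Searching refills the HUD list with a WB_ServerEntry per result, and joining takes a search result, with debug prints reporting attempts and failures.
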(event `self.ReceiveBeginPlay`
  (`|ExecutionSequence`
    (:`then_0`
      (bind _returnvalue (`|CreateWidget` "/Game/Blueprint/WB_HUD.WB_HUD_C"))
      (set `self.HUD` _returnvalue)
      (`UserWidget.AddToViewport` _returnvalue 0)
      (set `self.bShowMouseCursor` true))
    (:`then_1`
      (set `/Game/Blueprint/WB_HUD.PlayerController` self (`self.HUD`)))))

(event `CreateSession`
  (`CreateSessionCallbackProxyAdvanced.CreateAdvancedSession` :`PlayerController` self
    (:`OnSuccess`
      (`GameplayStatics.OpenLevelBySoftObjectPtr` "/Game/ThirdPerson/Maps/ThirdPersonMap.ThirdPersonMap" true "listen"))
    (:`OnFailure`
      (`KismetSystemLibrary.PrintString` "Failed to Create Session"))))

(event `GetListSession`
  (bind _results (`FindSessionsCallbackProxyAdvanced.FindSessionsAdvanced` self 0 false "AllServers")
    (:`then`
      (`KismetSystemLibrary.PrintString` "Attempt to find sessions"))
    (:`OnSuccess`
      (`/Game/Blueprint/WB_HUD.RemoveListSession` (`self.HUD`))
      (for _array_element _results
        (bind _returnvalue (`|CreateWidget` "/Game/Blueprint/WB_ServerEntry.WB_ServerEntry_C" null _array_element))
        (`/Game/Blueprint/WB_HUD.AddListSession` (`self.HUD`) _returnvalue)))
    (:`OnFailure`
      (`KismetSystemLibrary.PrintString` "Failed to find sessions"))))

(event `JoinSession`
  (params (SearchResult :type "BlueprintSessionResult Structure (by ref)"))
  (`JoinSessionCallbackProxy.JoinSession` self SearchResult
    (:`then`
      (`KismetSystemLibrary.PrintString` "Attempt to Join sessions"))
    (:`OnFailure`
      (`KismetSystemLibrary.PrintString` "Failed to Join Session"))))

(fn `UserConstructionScript`)